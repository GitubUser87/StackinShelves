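; Clickable shelf store point where the player drops off the box they are holding to earn points.
; BeginPlay enables click events on the player controller and caches the first-person character.
; Clicking the sphere with a box held teleports it to the sphere, clears the held reference, awards points and shrinks the box.
; The stored box is destroyed after a fixed delay.
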(event `self.ReceiveBeginPlay`
  ; Player Ref
  (set `PlayerController.bEnableClickEvents` true (`GameplayStatics.GetPlayerController` 0))
  (bind _asbp_first_person_character (cast `/Game/FirstPerson/Blueprints/BP_FirstPersonCharacter` (`GameplayStatics.GetPlayerCharacter` 0)))
  (set `self.PlayerRef` _asbp_first_person_character))

(event `self.Sphere.OnClicked`
  (params (TouchedComponent :type "PrimitiveComponent Object Reference") (ButtonPressed :type "Key Structure"))
  (bind _playerref (`self.PlayerRef`))
  (bind _heldbox (`/Game/FirstPerson/Blueprints/BP_FirstPersonCharacter.HeldBox` _playerref))
  ; Set Actor location
  (if (not (== _heldbox null))
    (`self.K2_SetActorLocation` _heldbox (`SceneComponent.K2_GetComponentLocation` (`self.Sphere`)) false true)
    (bind _output_get (set `self.Attached Actor` _heldbox))
    (set `/Game/FirstPerson/Blueprints/BP_FirstPersonCharacter.HeldBox` null _playerref)
    (`/Game/FirstPerson/Blueprints/BP_FirstPersonCharacter.AddPoints` _playerref)
    (`self.SetActorScale3D` _output_get (0.5 0.5 0.5))
    (`KismetSystemLibrary.Delay` 15.0)
    (`self.K2_DestroyActor` _output_get)))

(fn `UserConstructionScript`)