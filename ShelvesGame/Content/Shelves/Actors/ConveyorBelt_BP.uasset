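; ConveyorBelt_BP is a conveyor belt actor that moves whatever actors overlap its Box.
; A looping timer started at BeginPlay fires every tenth of a second and offsets each overlapping actor along the Arrow component's forward vector, without sweeping.
; Each step is Speed times the world's frame delta rather than the timer interval, so effective belt speed depends on frame rate.
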(event `self.ReceiveBeginPlay`
  ; Move Actors
  (`KismetSystemLibrary.K2_SetTimerDelegate` (delegate `Push`) 0.1 true))

(event `Push`
  ; Move Actors
  (for _array_element (`PrimitiveComponent.GetOverlappingActors` (`self.Box`) null)
    (`self.K2_AddActorWorldOffset` _array_element (* (`KismetMathLibrary.GetForwardVector` (`SceneComponent.K2_GetComponentRotation` (`self.Arrow`))) (* (`GameplayStatics.GetWorldDeltaSeconds`) (`self.Speed`))) false false)))

(fn `UserConstructionScript`)