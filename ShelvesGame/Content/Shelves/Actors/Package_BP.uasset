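; Clickable package actor that the first-person player selects as their held box until it is stored at a shelf point.
; BeginPlay caches the player, enables click events and allows selection after a short delay.
; Clicking sets the player's HeldBox to this package, adds a highlight overlay and plays a sound.
; Overlapping a StorePoint-tagged actor clears the overlay, stops physics simulation and disables further selection.
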(event `self.ReceiveBeginPlay`
  ; PlayerRef + Begin Functions
  (bind _asbp_first_person_character (cast `/Game/FirstPerson/Blueprints/BP_FirstPersonCharacter` (`GameplayStatics.GetPlayerCharacter` 0)))
  (set `self.PlayerRef` _asbp_first_person_character)
  (set `PlayerController.bEnableClickEvents` true (`GameplayStatics.GetPlayerController` 0))
  (`KismetSystemLibrary.Delay` 2.0)
  (set `self.Can?` true))

(event `self.Package.OnComponentBeginOverlap`
  (params (OverlappedComponent :type "PrimitiveComponent Object Reference") (OtherActor :type "Actor Object Reference") (OtherComp :type "PrimitiveComponent Object Reference") (OtherBodyIndex :type Integer) (bFromSweep :type Boolean) (SweepResult :type "HitResult Structure (by ref)"))
  (bind _package (`self.Package`))
  ; Stored
  (if (`self.ActorHasTag` OtherActor "StorePoint")
    (`MeshComponent.SetOverlayMaterial` _package null)
    (`PrimitiveComponent.SetSimulatePhysics` _package false)
    (set `self.Can?` false)))

(event `self.Package.OnClicked`
  (params (TouchedComponent :type "PrimitiveComponent Object Reference") (ButtonPressed :type "Key Structure"))
  ; On Clicked
  (if (`self.Can?`)
    (set `/Game/FirstPerson/Blueprints/BP_FirstPersonCharacter.HeldBox` self (`self.PlayerRef`))
    (`MeshComponent.SetOverlayMaterial` (`self.Package`) "/Game/Shelves/MAT/Highlight_MAT.Highlight_MAT")
    (`GameplayStatics.PlaySound2D` "/Engine/VREditor/Sounds/UI/Click_on_Button.Click_on_Button" 1.0 1.0 0.0 null null)))

(fn `UserConstructionScript`)