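; SpawnPoint_BP is a placed spawn point that keeps producing Package_BP_Child actors at its own transform.
; From BeginPlay a self-calling Spawn event loops on delays, spawning a package whenever the point is clear and waiting again when it is occupied.
; Overlap begin and end events on the Point component toggle the AtPoint flag, without filtering which actor overlaps.
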(event `self.ReceiveBeginPlay`
  ; SpawnActor
  (`self.Spawn`))

(event `Spawn`
  ; SpawnActor
  (`KismetSystemLibrary.Delay` 3.0)
  (if (`self.AtPoint`)
    (`KismetSystemLibrary.Delay` 3.0)
    (`self.Spawn`)
    (else
      (`|SpawnActorFromClass` "/Game/Shelves/Actors/Package_BP_Child.Package_BP_Child_C" (`self.GetTransform`) "Undefined" "MultiplyWithRoot" null null)
      (`KismetSystemLibrary.Delay` 3.0)
      (`self.Spawn`))))

(event `self.Point.OnComponentBeginOverlap`
  (params (OverlappedComponent :type "PrimitiveComponent Object Reference") (OtherActor :type "Actor Object Reference") (OtherComp :type "PrimitiveComponent Object Reference") (OtherBodyIndex :type Integer) (bFromSweep :type Boolean) (SweepResult :type "HitResult Structure (by ref)"))
  ; PointCheck
  (set `self.AtPoint` true))

(event `self.Point.OnComponentEndOverlap`
  (params (OverlappedComponent :type "PrimitiveComponent Object Reference") (OtherActor :type "Actor Object Reference") (OtherComp :type "PrimitiveComponent Object Reference") (OtherBodyIndex :type Integer))
  ; PointCheck
  (set `self.AtPoint` false))

(fn `UserConstructionScript`)