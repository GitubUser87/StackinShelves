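; Monster actor that hunts the player through timed teleports and ends the run with a jumpscare.
; It polls the player's Points until they equal two, then repeatedly teleports to one of three random locations, counting each timed move.
; On the seventh move it switches to the jumpscare camera, plays a sound and opens the main menu.
; A Reset event clears the count and hides the monster temporarily before movement resumes.
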(event `Loop`
  (if (`KismetMathLibrary.NearlyEqual_FloatFloat` (`/Game/FirstPerson/Blueprints/BP_FirstPersonCharacter.Points` (stale `self.ReceiveBeginPlay` _output_get)) 2.0) :!label _label
    (`/Engine/EditorBlueprintResources/StandardMacros.DoOnce` false
      (:`Completed`
        (`self.BeginMoving`)))
    (else
      (`KismetSystemLibrary.Delay` 0.2)
      (`self.Loop`))))

(event `self.ReceiveBeginPlay`
  (bind _asbp_first_person_character (cast `/Game/FirstPerson/Blueprints/BP_FirstPersonCharacter` (`GameplayStatics.GetPlayerCharacter` 0)))
  (bind _output_get (set `self.PlayerRef` _asbp_first_person_character))
  (set `self.Array` (`|MakeArray` (`self.Location 1`) (`self.Location 2`) (`self.Location 3`)))
  (goto _label))

(event `BeginMoving`
  (bind _array (`self.Array`))
  (`self.K2_SetActorLocation` (`|GetArrayItem` _array (`KismetMathLibrary.RandomIntegerInRange` 0 (`KismetArrayLibrary.Array_LastIndex` _array))) false true)
  (`KismetSystemLibrary.Delay` 10.0)
  (if (not (`self.Reset?`))
    (bind _result (`/Engine/EditorBlueprintResources/StandardMacros.IncrementInt` (`self.MovePoints`))
      (:`  `
        (set `self.MovePoints` _result)
        (`self.Jumpscare`)
        (`self.BeginMoving`)))))

(event `Reset`
  (set `self.Reset?` true)
  (set `self.MovePoints` 0)
  (`self.K2_SetActorLocation` (`self.HiddenLocation`) false true)
  (`KismetSystemLibrary.Delay` 15.0)
  (set `self.Reset?` false)
  (`self.BeginMoving`))

(event `Jumpscare`
  ; Jumpscare
  (if (== (`self.MovePoints`) 7)
    (`PlayerController.SetViewTargetWithBlend` (`GameplayStatics.GetPlayerController` 0) (`ActorComponent.GetOwner` (`self.JumpCam`)) 0.0 "VTBlend_Linear" 0.0 false)
    (`GameplayStatics.PlaySound2D` "/Engine/EditorSounds/Notifications/CompileFailed.CompileFailed" 1.0 1.0 0.0 null null)
    (`KismetSystemLibrary.Delay` 5.0)
    (`GameplayStatics.OpenLevel` "MainMenu")))

(fn `UserConstructionScript`)